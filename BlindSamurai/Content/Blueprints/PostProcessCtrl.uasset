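; Post-process controller that shows white and red (enemy) scan-line effects at given positions.
; Each show call cycles one of three slots per color, enables a tag-found PostProcessVolume and writes the position to that color's Material Parameter Collection.
; The position parameter's index is one step ahead of the volume's.
; A looping one-second Reset timer disables the previously recorded volume per color, then records the current one, delaying shutoff.
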(event `self.ReceiveBeginPlay`
  (`KismetSystemLibrary.K2_SetTimer` null "Reset" 1.0 true))

(fn `GetRedVolumeEnable`
  (params (index :type Integer))
  (returns (enable :type Boolean))
  (bind _outactors (`GameplayStatics.GetAllActorsWithTag` (`KismetStringLibrary.Conv_StringToName` (`KismetStringLibrary.Concat_StrStr` "PPE" (`KismetStringLibrary.Conv_IntToString` index)))))
  (bind _aspost_process_volume (cast `PostProcessVolume` (`|GetArrayItem` _outactors)))
  (return (`PostProcessVolume.bEnabled` _aspost_process_volume)))

(fn `GetWhiteVolumeEnable`
  (params (index :type Integer))
  (returns (enable :type Boolean))
  (bind _outactors (`GameplayStatics.GetAllActorsWithTag` (`KismetStringLibrary.Conv_StringToName` (`KismetStringLibrary.Concat_StrStr` "PP" (`KismetStringLibrary.Conv_IntToString` index)))))
  (bind _aspost_process_volume (cast `PostProcessVolume` (`|GetArrayItem` _outactors)))
  (return (`PostProcessVolume.bEnabled` _aspost_process_volume)))

(fn `Reset`
  ;[1 1 1] 白色扫描线重置
  (`self.SetWhiteVolumeEnable` (`self.PreLine`))
  (set `self.PreLine` (`self.CurLine`))
  ;[1 1 1] 红色扫描线重置
  (`self.Set Red Volume Enable` (`self.PreRedLine`))
  (set `self.PreRedLine` (`self.CurRedLine`)))

(fn `Set Red Volume Enable`
  (params (index :type Integer) (enable :type Boolean))
  (bind _outactors (`GameplayStatics.GetAllActorsWithTag` (`KismetStringLibrary.Conv_StringToName` (`KismetStringLibrary.Concat_StrStr` "PPE" (`KismetStringLibrary.Conv_IntToString` index)))))
  (bind _aspost_process_volume (cast `PostProcessVolume` (`|GetArrayItem` _outactors)))
  (set `PostProcessVolume.bEnabled` enable _aspost_process_volume))

(fn `SetEnable`
  (params (pp :type "PostProcessVolume Object Reference"))
  (set `PostProcessVolume.bEnabled` false pp)
  (return))

(fn `SetWhiteVolumeEnable`
  (params (index :type Integer) (enable :type Boolean))
  (bind _outactors (`GameplayStatics.GetAllActorsWithTag` (`KismetStringLibrary.Conv_StringToName` (`KismetStringLibrary.Concat_StrStr` "PP" (`KismetStringLibrary.Conv_IntToString` index)))))
  (bind _aspost_process_volume (cast `PostProcessVolume` (`|GetArrayItem` _outactors)))
  (set `PostProcessVolume.bEnabled` enable _aspost_process_volume))

(fn `ShowScanLineRed`
  (params (Pos :type "Vector Structure"))
  (bind _returnvalue (mod (+ (`self.CurRedLine`) 1) 3))
  (bind _output_get (set `self.CurRedLine` _returnvalue))
  (`self.Set Red Volume Enable` _output_get true)
  (`KismetMaterialLibrary.SetVectorParameterValue` "/Game/Effect/SL_Collection_enemy.SL_Collection_enemy" (`KismetStringLibrary.Conv_StringToName` (`KismetStringLibrary.Concat_StrStr` "Pos_0" (`KismetStringLibrary.Conv_IntToString` _returnvalue))) (`KismetMathLibrary.Conv_VectorToLinearColor` Pos))
  (return))

(fn `ShowScanLineWhite`
  (params (Pos :type "Vector Structure"))
  (bind _returnvalue (mod (+ (`self.CurLine`) 1) 3))
  (bind _output_get (set `self.CurLine` _returnvalue))
  (`self.SetWhiteVolumeEnable` _output_get true)
  (`KismetMaterialLibrary.SetVectorParameterValue` "/Game/Effect/SL_Collection.SL_Collection" (`KismetStringLibrary.Conv_StringToName` (`KismetStringLibrary.Concat_StrStr` "Pos_0" (`KismetStringLibrary.Conv_IntToString` _returnvalue))) (`KismetMathLibrary.Conv_VectorToLinearColor` Pos))
  (return))

(fn `UserConstructionScript`)