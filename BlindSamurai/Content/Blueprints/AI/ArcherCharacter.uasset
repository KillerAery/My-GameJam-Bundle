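; Archer enemy character Blueprint that periodically leaves droppings, can be outlined and ragdolls on death.
; A looping timer started at BeginPlay spawns a Shit actor at the archer's transform, linked back to it and living for one timer interval.
; Die decrements the game mode's enemy count, changes the animation state, detaches the controller and enables mesh physics.
; ShowOutline sets a material scalar, while ShootArrow is an empty stub.
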(event `self.ReceiveBeginPlay`
  (`KismetSystemLibrary.K2_SetTimerDelegate` (delegate `TakeShit`) (`self.TakeShitEverySeconds`) true))

(event `TakeShit`
  (bind _returnvalue (`|SpawnActorFromClass` "/Game/Blueprints/AI/Shit.Shit_C" (`self.GetTransform`) "Undefined" "OverrideRootScale" null null))
  (set `/Game/Blueprints/AI/Shit.enemy` self _returnvalue)
  (set `/Game/Blueprints/AI/Shit.lifetime` (`self.TakeShitEverySeconds`) _returnvalue))

(event `Die`
  (bind _mesh (`self.Mesh`))
  (bind _asanimation_test_game_mode (cast `/Game/Blueprints/GameMode/AnimationTestGameMode` (`GameplayStatics.GetGameMode`)))
  (`/Engine/EditorBlueprintResources/StandardMacros.DecrementInt` (`/Game/Blueprints/GameMode/AnimationTestGameMode.enemyNumber` _asanimation_test_game_mode)
    (:`  `
      (set `self.CurrentAnimState` "NewEnumerator0")
      (`self.DetachFromControllerPendingDestroy`)
      (`PrimitiveComponent.SetSimulatePhysics` _mesh true)
      (`PrimitiveComponent.SetCollisionEnabled` _mesh "QueryAndPhysics"))))

(fn `ShootArrow`)

(fn `ShowOutline`
  (`MeshComponent.SetScalarParameterValueOnMaterials` (`self.Mesh`) "Show" 1.0))

(fn `UserConstructionScript`)