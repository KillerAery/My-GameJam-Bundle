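; Game mode, named for animation testing, that shows a good-ending screen when its enemy count is zero.
; BeginPlay stores all ArcherCharacter actors and their count, which this file never updates afterwards.
; Tick checks that count and, if the HUD casts to BP_HUD, creates and adds a new good-end widget every frame it stays zero.
; A bad-end widget class is assigned but unused.
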(event `self.ReceiveBeginPlay`
  (set `self.GoodEndUI` "/Game/UMG/GoodEndTemplate.GoodEndTemplate_C")
  (set `self.BadEndUI` "/Game/UMG/BadEndTemplate.BadEndTemplate_C")
  (bind _outactors (`GameplayStatics.GetAllActorsOfClass` "/Game/Blueprints/AI/ArcherCharacter.ArcherCharacter_C"))
  (bind _output_get (set `self.enemies` _outactors))
  (set `self.enemyNumber` (`KismetArrayLibrary.Array_Length` _output_get)))

(event `self.ReceiveTick`
  (params (DeltaSeconds :type "Float (single-precision)"))
  (`/Engine/EditorBlueprintResources/StandardMacros.CompareInt` (`self.enemyNumber`)
    (:`==`
      (cast `/Game/UMG/BP_HUD` (`PlayerController.GetHUD` (`GameplayStatics.GetPlayerController` 0)))
      (bind _returnvalue (`|CreateWidget` (`self.GoodEndUI`)))
      (`UserWidget.AddToViewport` _returnvalue 0))))

(fn `UserConstructionScript`)